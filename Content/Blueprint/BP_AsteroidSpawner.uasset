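; BP_AsteroidSpawner is an actor meant to spawn BP_Asteroid actors from random positions along four sides of the play area.
; BeginPlay sets next-tick and looping random-interval timers with no visible bound event, spawns one asteroid, then randomly picks a side and offset for SpawnLocation.
; The nodes converting SpawnLocation into SpawnTransLocation are disconnected, so the spawn never receives the chosen position.
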(event EventBeginPlay
  (Class|KismetSystemLibrary|SetTimerforNextTickDelegate)
  (Utilities|Time|SetTimerbyEvent 0 (Math|Random|RandomFloatinRange 1.0 3.0) true)
  (Game|SpawnActorfromClass "/Game/Blueprint/BP_Asteroid.BP_Asteroid_C" (Variables|Default|GetSpawnTransLocation) "Undefined" "MultiplyWithRoot" 0 0)
  (switch int (Math|Random|RandomIntegerinRange 0 3)
    (:0
      (bind _output_get (Variables|Default|SetSpawnLocation (Math|Vector|MakeVector -2e+03 (Math|Random|RandomFloatinRange -1e+03 1e+03) 0.0))))
    (:1
      (bind _output_get_2 (Variables|Default|SetSpawnLocation (Math|Vector|MakeVector 2e+03 (Math|Random|RandomFloatinRange -1e+03 1e+03) 0.0))))
    (:2
      (bind _output_get_3 (Variables|Default|SetSpawnLocation (Math|Vector|MakeVector (Math|Random|RandomFloatinRange -1e+03 1e+03) 2e+03 0.0))))
    (:3
      (bind _output_get_4 (Variables|Default|SetSpawnLocation (Math|Vector|MakeVector (Math|Random|RandomFloatinRange -1e+03 1e+03) -2e+03 0.0))))))

(event Collision|EventActorBeginOverlap
  (params (OtherActor :type Actor%20Object%20Reference)))

(event EventTick
  (params (DeltaSeconds :type Float%20%28single-precision%29)))

(fn ConstructionScript)